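; BP_FartCloud is a growable gas cloud that affects the player and AI characters touching it.
; IncreaseSize scales the Cloud component up by a tenth per call and prints the new scale, while a separate CleanupTrigger destroys any BP_Fart entering it.
; Cloud overlaps damage AI once on entry and call the player UI's VignetteVisibility on both entry and exit.
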(event `IncreaseSize`
  (bind _cloud (`self.Cloud`))
  (bind _returnvalue (`SceneComponent.K2_GetComponentScale` _cloud))
  (`SceneComponent.SetWorldScale3D` _cloud (* _returnvalue 1.1))
  (`KismetSystemLibrary.PrintString` (`KismetStringLibrary.Conv_VectorToString` _returnvalue)))

(event `self.CleanupTrigger.OnComponentBeginOverlap`
  (params (OverlappedComponent :type "PrimitiveComponent Object Reference") (OtherActor :type "Actor Object Reference") (OtherComp :type "PrimitiveComponent Object Reference") (OtherBodyIndex :type Integer) (bFromSweep :type Boolean) (SweepResult :type "HitResult Structure (by ref)"))
  (bind _asbp_fart (cast `/Game/Blueprints/BP_Fart` OtherActor))
  (`self.K2_DestroyActor` _asbp_fart))

(event `self.Cloud.OnComponentBeginOverlap`
  (params (OverlappedComponent :type "PrimitiveComponent Object Reference") (OtherActor :type "Actor Object Reference") (OtherComp :type "PrimitiveComponent Object Reference") (OtherBodyIndex :type Integer) (bFromSweep :type Boolean) (SweepResult :type "HitResult Structure (by ref)"))
  (`|ExecutionSequence`
    (:`then_0`
      (bind _asbp_player (cast `/Game/ThirdPersonBP/Blueprints/BP_Player` OtherActor))
      (`/Game/Blueprints/Widgets/BP_PlayerUI.VignetteVisibility` (`/Game/ThirdPersonBP/Blueprints/BP_Player.UI` _asbp_player)))
    (:`then_1`
      (bind _asbp_ai (cast `/Game/AI/BP_AI` OtherActor))
      (`GameplayStatics.ApplyDamage` _asbp_ai 10.0))))

(event `self.Cloud.OnComponentEndOverlap`
  (params (OverlappedComponent :type "PrimitiveComponent Object Reference") (OtherActor :type "Actor Object Reference") (OtherComp :type "PrimitiveComponent Object Reference") (OtherBodyIndex :type Integer))
  (bind _asbp_player (cast `/Game/ThirdPersonBP/Blueprints/BP_Player` OtherActor))
  (`/Game/Blueprints/Widgets/BP_PlayerUI.VignetteVisibility` (`/Game/ThirdPersonBP/Blueprints/BP_Player.UI` _asbp_player)))

(fn `UserConstructionScript`)