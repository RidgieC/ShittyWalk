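; BP_Fart is a fart blast actor that knocks AI characters and a car away with a radial impulse.
; TriggerBox overlaps collect AI meshes, deal delayed damage and store the car's cube.
; Shortly after BeginPlay, it enables physics on those components and applies the impulse, far weaker for the car.
; It registers itself with every BP_AI; a separate Cleanup event, uncalled here, deregisters and destroys it after a delay.
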(event `ImpulseEvent`
  (`|ExecutionSequence`
    (:`then_0`
      (for _array_element (`self.AIMesh`)
        (`/Engine/EditorBlueprintResources/StandardMacros.IsValid` _array_element
          (:`Is Valid`
            (`PrimitiveComponent.SetSimulatePhysics` _array_element true)
            (`self.RadialForce` _array_element (`self.FartStrength`))))))
    (:`then_1`
      (bind _cube (`self.Cube`)
        (:`then`
          (`PrimitiveComponent.SetSimulatePhysics` _cube true)
          (`self.RadialForce` _cube (* (`self.FartStrength`) 0.05)))
        (:`else`)))))

(event `self.ReceiveBeginPlay`
  (`self.SetupFartCheck`)
  (`KismetSystemLibrary.Delay` 0.1)
  (`self.ImpulseEvent`))

(event `SetupFartCheck`
  (bind _outactors (`GameplayStatics.GetAllActorsOfClass` "/Game/AI/BP_AI.BP_AI_C"))
  (for _array_element _outactors
    (bind _returnvalue (`KismetArrayLibrary.Array_Add` (`/Game/AI/BP_AI.Fart` _array_element) self))
    (set `self.FartIndex` _returnvalue)))

(event `Cleanup`
  (`KismetSystemLibrary.Delay` 5.0)
  (bind _outactors (`GameplayStatics.GetAllActorsOfClass` "/Game/AI/BP_AI.BP_AI_C"))
  (for _array_element _outactors
    (`KismetArrayLibrary.Array_Remove` (`/Game/AI/BP_AI.Fart` _array_element) (`self.FartIndex`)))
  (`KismetSystemLibrary.Delay` 0.2)
  (`self.K2_DestroyActor`))

(event `self.TriggerBox.OnComponentBeginOverlap`
  (params (OverlappedComponent :type "PrimitiveComponent Object Reference") (OtherActor :type "Actor Object Reference") (OtherComp :type "PrimitiveComponent Object Reference") (OtherBodyIndex :type Integer) (bFromSweep :type Boolean) (SweepResult :type "HitResult Structure (by ref)"))
  (`|ExecutionSequence`
    (:`then_0`
      (bind _asbp_ai (cast `/Game/AI/BP_AI` OtherActor))
      (`KismetArrayLibrary.Array_Add` (`self.AIMesh`) (`Character.Mesh` _asbp_ai))
      (`KismetSystemLibrary.Delay` 0.1)
      (`GameplayStatics.ApplyDamage` _asbp_ai 10.0))
    (:`then_1`
      (bind _asbp_car (cast `/Game/Blueprints/BP_Car` OtherActor))
      (set `self.Cube` (`/Game/Blueprints/BP_Car.Cube` _asbp_car)))))

(fn `RadialForce`
  (params (Target :type "PrimitiveComponent Object Reference") (Strength :type "Float (double-precision)"))
  (`PrimitiveComponent.AddRadialImpulse` Target (`SceneComponent.K2_GetComponentLocation` (`self.TriggerBox`)) (`self.FartRadius`) Strength "RIF_Linear" true))

(fn `UserConstructionScript`)