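; BP_ToiletTrigger is a trigger actor that serves as a win check and an AI spawner when the player passes through it.
; On player overlap it only prints a game-finished or play-sound placeholder, depending on Free.
; When the player leaves a non-Free trigger, a self-calling, delayed Spawner creates BP_AI at the actor's transform until NumberOfAI is reached, handing each a start location object.
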(event `SetStartLocation`
  (bind _output_get (set `self.HasStartLocation` true))
  (`/Game/AI/BP_AI.AssignStartLocation` (`self.SpawnedAI`) (`self.StartLocationObject`) _output_get))

(event `GameWonState`
  (if (`self.Free`)
    (`KismetSystemLibrary.PrintString` "Game finished" true true (struct :`R` 1.0 :`B` 0.908446 :`A` 1.0) 10.0)
    (else
      (`KismetSystemLibrary.PrintString` "Play sound"))))

(event `self.Trigger.OnComponentBeginOverlap`
  (params (OverlappedComponent :type "PrimitiveComponent Object Reference") (OtherActor :type "Actor Object Reference") (OtherComp :type "PrimitiveComponent Object Reference") (OtherBodyIndex :type Integer) (bFromSweep :type Boolean) (SweepResult :type "HitResult Structure (by ref)"))
  (if (== (`GameplayStatics.GetObjectClass` OtherActor) "/Game/ThirdPersonBP/Blueprints/BP_Player.BP_Player_C")
    (`self.GameWonState`)))

(event `self.Trigger.OnComponentEndOverlap`
  (params (OverlappedComponent :type "PrimitiveComponent Object Reference") (OtherActor :type "Actor Object Reference") (OtherComp :type "PrimitiveComponent Object Reference") (OtherBodyIndex :type Integer))
  (if (== (`GameplayStatics.GetObjectClass` OtherActor) "/Game/ThirdPersonBP/Blueprints/BP_Player.BP_Player_C")
    (if (not (`self.Free`))
      (`self.Spawner`))))

(event `Spawner`
  (if (not (`self.HasSpawned`))
    (bind _returnvalue (`|SpawnActorFromClass` "/Game/AI/BP_AI.BP_AI_C" (`self.GetTransform`) "Undefined" "OverrideRootScale" null null))
    (set `self.SpawnedAI` _returnvalue)
    (`self.SetStartLocation`)
    (if (== (`self.CurrentAINumber`) (`self.NumberOfAI`))
      (set `self.HasSpawned` true)
      (else
        (`KismetSystemLibrary.Delay` (`self.SpawnDelay`))
        (set `self.CurrentAINumber` (+ (`self.CurrentAINumber`) 1))
        (`self.Spawner`)))))

(fn `UserConstructionScript`)