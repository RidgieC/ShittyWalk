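; BP_SpawnTrigger is a trigger actor that spawns a series of AI enemies when BP_Player overlaps it and plays a shout sound.
; Spawner re-calls itself after a delay until the configured AI count is reached, then sets HasSpawned to block further spawns.
; Spawn location and rotation come from separate random picks among the spawn objects.
; Each AI receives a start location object indexed by another random roll over that array's range.
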(event `SetStartLocation`
  (bind _output_get (set `self.HasStartLocation` true))
  (`/Game/AI/BP_AI.AssignStartLocation` (`self.SpawnedAI`) (`|GetArrayItem` (`self.StartLocationObject`) (`self.LocationNumber`)) _output_get))

(event `self.Trigger.OnComponentBeginOverlap`
  (params (OverlappedComponent :type "PrimitiveComponent Object Reference") (OtherActor :type "Actor Object Reference") (OtherComp :type "PrimitiveComponent Object Reference") (OtherBodyIndex :type Integer) (bFromSweep :type Boolean) (SweepResult :type "HitResult Structure (by ref)"))
  (if (== (`GameplayStatics.GetObjectClass` OtherActor) "/Game/ThirdPersonBP/Blueprints/BP_Player.BP_Player_C")
    (`self.Spawner`)
    (`GameplayStatics.SpawnSoundAtLocation` "/Game/Sound/Angry_Hey.Angry_Hey" (`self.K2_GetActorLocation`) (struct) 1.0 1.0 0.0 null null)))

(event `Spawner`
  (bind _spawnlocationobject (`self.SpawnlocationObject`))
  (bind _returnvalue (`KismetMathLibrary.RandomIntegerInRange` 0 (- (`KismetArrayLibrary.Array_Length` _spawnlocationobject) 1)))
  (bind (_returnvalue_location _returnvalue_rotation) (`KismetMathLibrary.BreakTransform` (`self.GetTransform` (`|GetArrayItem` _spawnlocationobject _returnvalue))))
  (set `self.LocationNumber` _returnvalue)
  (if (not (`self.HasSpawned`))
    (bind _returnvalue_2 (`|SpawnActorFromClass` "/Game/AI/BP_AI.BP_AI_C" (`KismetMathLibrary.MakeTransform` _returnvalue_location _returnvalue_rotation) "Undefined" "OverrideRootScale" null null))
    (set `self.SpawnedAI` _returnvalue_2)
    (`self.SetStartLocation`)
    (if (== (`self.CurrentAINumber`) (- (`self.NumberOfAI`) 1))
      (set `self.HasSpawned` true)
      (else
        (`KismetSystemLibrary.Delay` (`self.SpawnDelay`))
        (set `self.CurrentAINumber` (+ (`self.CurrentAINumber`) 1))
        (`self.Spawner`)))))

(fn `UserConstructionScript`)