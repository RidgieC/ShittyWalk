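; Toilet manager that marks one randomly chosen trigger in its ToiletTriggers array as free, starting at BeginPlay.
; CheckOccupancy makes the pick and starts a one-shot, minute-long timer, whose bound event is not named but is presumably ResetToilet.
; ResetToilet clears Free on the triggers and calls CheckOccupancy again through a short Delay placed inside the loop.
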(event `self.ReceiveBeginPlay`
  (`self.CheckOccupancy`))

(event `CheckOccupancy`
  (bind _output_get (set `self.ToiletNumber` (`KismetMathLibrary.RandomIntegerInRange` 0 (- (`KismetArrayLibrary.Array_Length` (`self.ToiletTriggers`)) 1))))
  (set `/Game/Blueprints/BP_ToiletTrigger.Free` true (`|ConvertAsset` (`|GetArrayItem` (`self.ToiletTriggers`) _output_get)))
  (`KismetSystemLibrary.K2_SetTimerDelegate` (`|CreateDelegate` :!event `ResetToilet`) 60.0))

(event `ResetToilet`
  (for _array_element (`self.ToiletTriggers`)
    (set `/Game/Blueprints/BP_ToiletTrigger.Free` false (`|ConvertAsset` _array_element))
    (`KismetSystemLibrary.Delay` 0.2)
    (`self.CheckOccupancy`)))

(fn `UserConstructionScript`)