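; BP_AI is an NPC character with randomised shirt and hair materials that punches the player and enters a death state on any damage.
; It hands BP_AIController its behavior tree, player target and optional start location.
; A delayed Tick passes the newest valid Fart to the controller.
; Attack opens a timed window in which the fist-socket collider damages the player; an older material-variation chain is left unconnected.
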(event `AssignStartLocation`
  (params (StartLocationObject :type "Actor Object Reference") (HasStartLocation :type Boolean))
  (`/Game/AI/BP_AIController.SetupAIC` (`self.AIController`) (`self.BT`) (`GameplayStatics.GetPlayerPawn` 0) StartLocationObject HasStartLocation))

(event `self.ReceiveBeginPlay`
  (bind _mesh (`self.Mesh`))
  (bind _mesh_2 (`self.Mesh`))
  (bind _asbp_aicontroller (cast `/Game/AI/BP_AIController` (`AIBlueprintHelperLibrary.GetAIController` self)))
  (bind _output_get (set `self.AIController` _asbp_aicontroller))
  (`/Game/AI/BP_AIController.SetupAIC` _output_get (`self.BT`) (`GameplayStatics.GetPlayerPawn` 0) null false)
  (`SceneComponent.K2_AttachToComponent` (`self.PunchCollider`) (`self.Mesh`) "Fist_Socket" "SnapToTarget" "SnapToTarget" "KeepWorld" true)
  (switch `int` (`KismetMathLibrary.RandomIntegerInRange` 0 3)
    (:`0`
      (`PrimitiveComponent.SetMaterial` _mesh 0 "/Game/Mannequin/Character/Fatman/CharacterVariationMaterials/M_RedShirt.M_RedShirt"))
    (:`1`
      (`PrimitiveComponent.SetMaterial` _mesh 0 "/Game/Mannequin/Character/Fatman/CharacterVariationMaterials/M_BlueShirt.M_BlueShirt"))
    (:`2`
      (`PrimitiveComponent.SetMaterial` _mesh 0 "/Game/Mannequin/Character/Fatman/CharacterVariationMaterials/M_BrownShirt.M_BrownShirt"))
    (:`3`
      (`PrimitiveComponent.SetMaterial` _mesh 0 "/Game/Mannequin/Character/Fatman/CharacterVariationMaterials/M_GreenShirt.M_GreenShirt")))
  (switch `int` (`KismetMathLibrary.RandomIntegerInRange` 0 2)
    (:`0`
      (`PrimitiveComponent.SetMaterial` _mesh_2 4 "/Game/Mannequin/Character/Fatman/CharacterVariationMaterials/M_BlackHair.M_BlackHair"))
    (:`1`
      (`PrimitiveComponent.SetMaterial` _mesh_2 4 "/Game/Mannequin/Character/Fatman/CharacterVariationMaterials/M_BlondeHair.M_BlondeHair"))
    (:`2`
      (`PrimitiveComponent.SetMaterial` _mesh_2 4 "/Game/Mannequin/Character/Fatman/CharacterVariationMaterials/M_BrownHair.M_BrownHair"))))

(event `CheckFarts`
  (bind _fart (`self.Fart`))
  (bind _output (`|GetArrayItem` _fart (`KismetArrayLibrary.Array_LastIndex` _fart)))
  (`/Engine/EditorBlueprintResources/StandardMacros.IsValid` _output
    (:`Is Valid`
      (`/Game/AI/BP_AIController.SetupFartAIC` (`self.AIController`) _output))))

(event `self.ReceiveTick`
  (params (DeltaSeconds :type "Float (single-precision)"))
  (`KismetSystemLibrary.Delay` 0.5)
  (`self.CheckFarts`))

(event `Attack`
  (set `self.Attacking` true)
  (`GameplayStatics.SpawnSoundAtLocation` "/Game/Sound/Punch.Punch" (`self.K2_GetActorLocation`) (struct) 1.0 1.0 0.0 null null)
  (`KismetSystemLibrary.Delay` 1.0)
  (set `self.Attacking` false))

(event `self.ReceiveAnyDamage`
  (params (Damage :type "Float (single-precision)") (DamageType :type "DamageType Object Reference") (InstigatedBy :type "Controller Object Reference") (DamageCauser :type "Actor Object Reference"))
  (`KismetSystemLibrary.PrintString` "Damage" true true (struct :`R` 1.0 :`B` 0.03671 :`A` 1.0))
  (`/Game/AI/BP_AIController.DeathState` (`self.AIController`)))

(event `self.PunchCollider.OnComponentBeginOverlap`
  (params (OverlappedComponent :type "PrimitiveComponent Object Reference") (OtherActor :type "Actor Object Reference") (OtherComp :type "PrimitiveComponent Object Reference") (OtherBodyIndex :type Integer) (bFromSweep :type Boolean) (SweepResult :type "HitResult Structure (by ref)"))
  (if (== (`GameplayStatics.GetObjectClass` OtherActor) "/Game/ThirdPersonBP/Blueprints/BP_Player.BP_Player_C")
    (if (`self.Attacking`)
      (`GameplayStatics.ApplyDamage` (`GameplayStatics.GetPlayerPawn` 0) 10.0))))

(fn `ChangeVariation`
  (params (MaterialIndex :type Integer) (Material :type "MaterialInterface Object Reference"))
  (`PrimitiveComponent.SetMaterial` (`self.Mesh`) MaterialIndex Material)
  (bind _output_get (set `self.MaterialIndex` (+ (`self.MaterialIndex`) 1)))
  (`KismetSystemLibrary.PrintString` (`KismetStringLibrary.Conv_IntToString` _output_get)))

(fn `UserConstructionScript`
  (`SceneComponent.K2_AttachToComponent` (`self.PunchCollider`) (`self.Mesh`) "Fist_Socket" "SnapToTarget" "SnapToTarget" "KeepWorld" true))